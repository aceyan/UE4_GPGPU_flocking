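; Test actor that seeds position and velocity render targets on BeginPlay.
; It creates a dynamic instance of InitializeRT_mat and draws it into PositionRT using Range from the material parameter collection.
; It stores that Range, then reuses the instance with a fixed Range to fill VelocityRT.
; The Blueprint has no per-frame logic, only this one-time GPU-side initialization.
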(event EventBeginPlay
  ;[1 1 1] initialization
  (Utilities|FlowControl|Sequence
    (:then_0
      (bind _returnvalue (Rendering|Material|CreateDynamicMaterialInstance "/Game/Materials/InitializeRT_mat.InitializeRT_mat" "None" :!class /Script/Engine.KismetMaterialLibrary))
      (Variables|Default|SetInitialziePosAndVelocity_mat _returnvalue))
    (:then_1
      (bind _returnvalue_2 (Rendering|Material|GetScalarParameterValue "/Game/Materials/ParametersCollection.ParametersCollection" "Range" :!class /Script/Engine.KismetMaterialLibrary))
      (Rendering|Material|SetScalarParameterValue (Variables|Default|GetInitialziePosAndVelocity_mat) "Range" _returnvalue_2 :!class /Script/Engine.MaterialInstanceDynamic)
      (Rendering|DrawMaterialtoRenderTarget "/Game/Materials/PositionRT.PositionRT" (Variables|Default|GetInitialziePosAndVelocity_mat))
      (Variables|Default|SetRange _returnvalue_2)
      (Rendering|Material|SetScalarParameterValue (Variables|Default|GetInitialziePosAndVelocity_mat) "Range" 2.0 :!class /Script/Engine.MaterialInstanceDynamic)
      (Rendering|DrawMaterialtoRenderTarget "/Game/Materials/VelocityRT.VelocityRT" (Variables|Default|GetInitialziePosAndVelocity_mat)))))

(event EventTick
  (params (DeltaSeconds :type Float%20%28single-precision%29)))

(fn ConstructionScript)