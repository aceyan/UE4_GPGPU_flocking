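; BP_Player is a player Blueprint that adjusts the instance count of a referenced InstancedActor at runtime, apparently for testing instancing.
; Keys 1 and 2 read the current count and re-initialize the instances with 1000 fewer or 1000 more, with no clamping in this Blueprint.
; BeginPlay, overlap, Tick and the construction script do nothing.
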(event EventBeginPlay)

(event Collision|EventActorBeginOverlap
  (params (OtherActor :type Actor%20Object%20Reference)))

(event EventTick
  (params (DeltaSeconds :type Float%20%28single-precision%29)))

(event Input|KeyboardEvents|2
  (params (Key :type Key%20Structure :default "None"))
  ;[1 1 1] increase instance num
  (:Pressed
    (bind _returnvalue (Class|InstancingRootActor|GetInstanceCount (Variables|Default|GetInstancedActor)))
    (Class|InstancingRootActor|InitInstances (Variables|Default|GetInstancedActor) (+ _returnvalue 1000))))

(event Input|KeyboardEvents|1
  (params (Key :type Key%20Structure :default "None"))
  ;[1 1 1] decrease instance num
  (:Pressed
    (bind _returnvalue (Class|InstancingRootActor|GetInstanceCount (Variables|Default|GetInstancedActor)))
    (Class|InstancingRootActor|InitInstances (Variables|Default|GetInstancedActor) (- _returnvalue 1000))))

(fn ConstructionScript)