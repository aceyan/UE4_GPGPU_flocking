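; Actor that runs a GPU simulation of positions and velocities stored in render targets.
; BeginPlay creates dynamic velocity and position update materials and clears two render target pairs to black.
; Each Tick runs two ping-pong steps between the pairs, drawing new velocity first and then feeding it into the position pass.
; The second step writes back into the first pair, so results always end there for the next frame.
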(event EventBeginPlay
  (Utilities|FlowControl|Sequence
    (:then_0
      (bind _returnvalue (Rendering|Material|CreateDynamicMaterialInstance "/Game/Materials/PositionUpdate_mat.PositionUpdate_mat" "None" :!class /Script/Engine.KismetMaterialLibrary))
      (Variables|Default|SetUpdatePosition_mat _returnvalue))
    (:then_1
      (bind _returnvalue_2 (Rendering|Material|CreateDynamicMaterialInstance "/Game/Materials/VelocityUpdate_mat.VelocityUpdate_mat" "None" :!class /Script/Engine.KismetMaterialLibrary))
      (Variables|Default|SetUpdateVelocity_mat _returnvalue_2))
    (:then_2
      (Rendering|ClearRenderTarget2D "/Game/Materials/Position_RT1.Position_RT1")
      (Rendering|ClearRenderTarget2D "/Game/Materials/Velocity_RT1.Velocity_RT1")
      (Rendering|ClearRenderTarget2D "/Game/Materials/Position_RT2.Position_RT2")
      (Rendering|ClearRenderTarget2D "/Game/Materials/Velocity_RT2.Velocity_RT2"))))

(event Collision|EventActorBeginOverlap
  (params (OtherActor :type Actor%20Object%20Reference)))

(event EventTick
  (params (DeltaSeconds :type Float%20%28single-precision%29))
  (bind _updatevelocity_mat (Variables|Default|GetUpdateVelocity_mat))
  (bind _updateposition_mat (Variables|Default|GetUpdatePosition_mat))
  (bind _updatevelocity_mat_2 (Variables|Default|GetUpdateVelocity_mat))
  (bind _updateposition_mat_2 (Variables|Default|GetUpdatePosition_mat))
  (Utilities|FlowControl|Sequence
    (:then_0
      (Rendering|Material|SetTextureParameterValue _updatevelocity_mat_2 "Position_RT" "/Game/Materials/Position_RT1.Position_RT1")
      (Rendering|Material|SetTextureParameterValue _updatevelocity_mat_2 "Velocity_RT" "/Game/Materials/Velocity_RT1.Velocity_RT1")
      (Rendering|DrawMaterialtoRenderTarget "/Game/Materials/Velocity_RT2.Velocity_RT2" _updatevelocity_mat_2))
    (:then_1
      (Rendering|Material|SetTextureParameterValue _updateposition_mat_2 "Position_RT" "/Game/Materials/Position_RT1.Position_RT1")
      (Rendering|Material|SetTextureParameterValue _updateposition_mat_2 "Velocity_RT" "/Game/Materials/Velocity_RT2.Velocity_RT2")
      (Rendering|DrawMaterialtoRenderTarget "/Game/Materials/Position_RT2.Position_RT2" _updateposition_mat_2))
    (:then_2
      (Rendering|Material|SetTextureParameterValue _updatevelocity_mat "Position_RT" "/Game/Materials/Position_RT2.Position_RT2")
      (Rendering|Material|SetTextureParameterValue _updatevelocity_mat "Velocity_RT" "/Game/Materials/Velocity_RT2.Velocity_RT2")
      (Rendering|DrawMaterialtoRenderTarget "/Game/Materials/Velocity_RT1.Velocity_RT1" _updatevelocity_mat))
    (:then_3
      (Rendering|Material|SetTextureParameterValue _updateposition_mat "Position_RT" "/Game/Materials/Position_RT2.Position_RT2")
      (Rendering|Material|SetTextureParameterValue _updateposition_mat "Velocity_RT" "/Game/Materials/Velocity_RT1.Velocity_RT1")
      (Rendering|DrawMaterialtoRenderTarget "/Game/Materials/Position_RT1.Position_RT1" _updateposition_mat))))

(fn ConstructionScript)